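; Base death gameplay ability that puts the avatar pawn through its death animation.
; On activation it unpossesses the pawn's controller, plays a configurable montage and ends when the montage completes, blends out, is interrupted or is cancelled.
; Ending the ability pauses animations and disables anim curves on the owning skeletal mesh, freezing the pose.
; The actor stays in the world, as the destroy node is disconnected.
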(event Ability|EventActivateAbility
  (Pawn|UnPossess (Pawn|GetController (.AsPawn (Utilities|Casting|CastToPawn (Ability|GetAvatarActorfromActorInfo)))))
  (|PlayMontageandWaitProxy "None" (Variables|Default|GetMontage%20to%20Play) 1.0 "None" true 1.0 0.0 false
    (:OnCompleted
      _)
    (:OnBlendOut
      _)
    (:OnInterrupted
      _)
    (:OnCancelled
      _))
  (Ability|EndAbility))

(event Ability|EventOnEndAbility
  (params (bWasCancelled :type Boolean))
  (bind _returnvalue (Class|GameplayAbility|GetOwningComponentfromActorInfo))
  (Variables|/Script/Engine.SkeletalMeshComponent|SetbPauseAnims _returnvalue true)
  (Class|SkeletalMeshComponent|SetDisableAnimCurves _returnvalue true))